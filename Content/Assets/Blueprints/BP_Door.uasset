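; BP_Door is a double door that swings open when a BP_ThirdPersonController actor overlaps its trigger box.
; The DoorsOpening timeline yaws the left and right leaves in opposite directions, then sets Open to block further triggers.
; The E key sets a Pressed flag, but its check is unconnected, so opening needs no key press and nothing closes the door.
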(event `Key|E`
  (params (Key :type "Key Structure"))
  (:`Pressed`
    (set `self.Pressed` true))
  (:`Released`
    (set `self.Pressed` false)))

(event `self.Trigger_box.OnComponentBeginOverlap`
  (params (OverlappedComponent :type "PrimitiveComponent Object Reference") (OtherActor :type "Actor Object Reference") (OtherComp :type "PrimitiveComponent Object Reference") (OtherBodyIndex :type Integer) (bFromSweep :type Boolean) (SweepResult :type "HitResult Structure (by ref)"))
  (if (not (`self.Open`))
    (cast `/Game/Assets/Blueprints/BP_ThirdPersonController` OtherActor)
    (bind (_direction _opendoors) (`Timeline|DoorsOpening`)
      (:`Update`
        (bind _returnvalue (`KismetMathLibrary.MakeRotator` 0.0 0.0 _opendoors))
        (`SceneComponent.K2_SetRelativeRotation` (`self.Door_left`) _returnvalue false false)
        (`SceneComponent.K2_SetRelativeRotation` (`self.Door_Right`) (* _returnvalue -1.0) false false))
      (:`Finished`
        (set `self.Open` true)))))

(fn `UserConstructionScript`)